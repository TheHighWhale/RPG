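; Player stats component that tracks current and max health and stamina on BP_ThirdPersonCharacter.
; One tick after BeginPlay it caches the owner and fills its HUD bars.
; Functions adjust values and bars, though Increase Health and Increase Stamina refresh bars only when clamping.
; Stamina logic is miswired: Increase Stamina writes CurrentHealth, Increase Max Stamina zeroes the maximum, and Decrease Stamina returns whether health is depleted.
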(event `self.ReceiveBeginPlay`
  (`KismetSystemLibrary.DelayUntilNextTick`)
  (bind _asbp_third_person_character (cast `/Game/ThirdPerson/Blueprints/BP_ThirdPersonCharacter` (`self.GetOwner`)))
  (set `self.Player Character BP` _asbp_third_person_character)
  (`ProgressBar.SetPercent` (`/Game/UI/WBP_HUD.StaminaBar` (`/Game/ThirdPerson/Blueprints/BP_ThirdPersonCharacter.HUD Widget` (`self.Player Character BP`))) (/ (`self.currentStamina`) (`self.maxStamina`)))
  (`ProgressBar.SetPercent` (`/Game/UI/WBP_HUD.HealthBar` (`/Game/ThirdPerson/Blueprints/BP_ThirdPersonCharacter.HUD Widget` (`self.Player Character BP`))) (/ (`self.currentHealth`) (`self.maxHealth`))))

(fn `Decrease Health`
  (params (Damage :type "Float (double-precision)"))
  (returns (`IsPlayerDead?` :type Boolean))
  (if (not (<= (`self.currentHealth`) 0.0))
    (bind _output_get (set `self.currentHealth` (- (`self.currentHealth`) Damage)))
    (`ProgressBar.SetPercent` (`/Game/UI/WBP_HUD.HealthBar` (`/Game/ThirdPerson/Blueprints/BP_ThirdPersonCharacter.HUD Widget` (`self.Player Character BP`))) (/ _output_get (`self.maxHealth`)))
    (if (<= (`self.currentHealth`) 0.0)
      _
      (else
        (return false))))
  (return true))

(fn `Decrease Stamina`
  (params (StaminaDepleted :type "Float (double-precision)"))
  (returns (DeadNoStamina :type Boolean))
  (bind _output_get (set `self.currentStamina` (- (`self.currentStamina`) StaminaDepleted)))
  (`ProgressBar.SetPercent` (`/Game/UI/WBP_HUD.StaminaBar` (`/Game/ThirdPerson/Blueprints/BP_ThirdPersonCharacter.HUD Widget` (`self.Player Character BP`))) (/ _output_get (`self.maxStamina`)))
  (if (<= (`self.currentHealth`) 0.0)
    (return true)
    (else
      (return false))))

(fn `Increase Health`
  (params (AddedHealth :type "Float (double-precision)"))
  (set `self.currentHealth` (+ (`self.currentHealth`) AddedHealth))
  (if (> (`self.currentHealth`) (`self.maxHealth`))
    (bind _output_get (set `self.currentHealth` (`self.maxHealth`)))
    (`ProgressBar.SetPercent` (`/Game/UI/WBP_HUD.HealthBar` (`/Game/ThirdPerson/Blueprints/BP_ThirdPersonCharacter.HUD Widget` (`self.Player Character BP`))) (/ _output_get (`self.maxHealth`)))))

(fn `Increase Max Health`
  (params (`Health Increment` :type "Float (double-precision)"))
  (bind _output_get (set `self.maxHealth` (+ (`self.maxHealth`) `Health Increment`)))
  (bind _output_get_2 (set `self.currentHealth` _output_get))
  (`ProgressBar.SetPercent` (`/Game/UI/WBP_HUD.HealthBar` (`/Game/ThirdPerson/Blueprints/BP_ThirdPersonCharacter.HUD Widget` (`self.Player Character BP`))) (/ _output_get_2 (`self.maxHealth`))))

(fn `Increase Max Stamina`
  (params (AddStamina :type "Float (double-precision)"))
  (bind _output_get (set `self.maxStamina` 0.0))
  (bind _output_get_2 (set `self.currentStamina` _output_get))
  (`ProgressBar.SetPercent` (`/Game/UI/WBP_HUD.StaminaBar` (`/Game/ThirdPerson/Blueprints/BP_ThirdPersonCharacter.HUD Widget` (`self.Player Character BP`))) (/ _output_get_2 (`self.maxStamina`))))

(fn `Increase Stamina`
  (params (AddedStamina :type "Float (double-precision)"))
  (set `self.currentHealth` (+ (`self.currentStamina`) AddedStamina))
  (if (> (`self.currentStamina`) (`self.maxStamina`))
    (bind _output_get (set `self.currentStamina` (`self.maxStamina`)))
    (`ProgressBar.SetPercent` (`/Game/UI/WBP_HUD.StaminaBar` (`/Game/ThirdPerson/Blueprints/BP_ThirdPersonCharacter.HUD Widget` (`self.Player Character BP`))) (/ _output_get (`self.maxStamina`)))))