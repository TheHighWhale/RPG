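; Actor component that runs a four-step melee combo, three attacks and a kick, on the owning BP_ThirdPersonCharacter's mesh.
; Attack input, gated by CanAttack, plays the montage for the current AttackIndex or buffers the press while IsAttacking.
; SwordAttackCombo plays the next step if a press was buffered, otherwise resets the combo.
; Each step has a DoOnce guard and short delay; nothing here sets IsAttacking true or calls SwordAttackCombo.
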(event `self.ReceiveBeginPlay`
  (bind _asbp_third_person_character (cast `/Game/ThirdPerson/Blueprints/BP_ThirdPersonCharacter` (`self.GetOwner`)))
  (set `self.characterMesh` (`Character.Mesh` _asbp_third_person_character)))

(event `InputAction|Attack`
  (params (Key :type "Key Structure"))
  ;[0.05098 0.05098 0.05098] Attack Input
  (:`Pressed`
    (if (`self.canAttack?`)
      (`self.Sword Attack`))))

(event `Sword Attack`
  ;[0.05098 0.05098 0.05098] Sword Attack
  (if (`self.isAttacking?`)
    (set `self.saveAttack?` true)
    (else
      (set `self.saveAttack?` false)
      (switch `int` (`self.attackIndex`) :!label _label
        (:`0`
          (`self.Attack 1`))
        (:`1`
          (`self.Attack 2`))
        (:`2`
          (`self.Attack 3`))
        (:`3`
          (`self.Attack 4`))))))

(event `Sword Attack Combo`
  ;[0.05098 0.05098 0.05098] Continue combo
  (if (`self.saveAttack?`)
    (set `self.saveAttack?` false)
    (goto _label)
    (else
      (`self.Stop Combo`))))

(event `Stop Combo`
  ;[0.05098 0.05098 0.05098] Stop combo
  (set `self.isAttacking?` false)
  (set `self.attackIndex` 0))

(event `Attack 1`
  ;[0.05098 0.05098 0.05098] Attack 1
  (`/Engine/EditorBlueprintResources/StandardMacros.DoOnce` false :!label _label_2
    (:`Completed`
      (`KismetSystemLibrary.Delay` 0.1)
      (`|PlayMontage` (`self.characterMesh`) "/Game/Animation/Sword_Attacks/Attack1_Montage.Attack1_Montage"
        (:`then`
          (set `self.attackIndex` 1)
          (goto _label_2 :!via `Reset`))))))

(event `Attack 2`
  ;[0.05098 0.05098 0.05098] Attack 2
  (`/Engine/EditorBlueprintResources/StandardMacros.DoOnce` false :!label _label_3
    (:`Completed`
      (`KismetSystemLibrary.Delay` 0.1)
      (`|PlayMontage` (`self.characterMesh`) "/Game/Animation/Sword_Attacks/Attack2_Montage.Attack2_Montage"
        (:`then`
          (set `self.attackIndex` 2)
          (goto _label_3 :!via `Reset`))))))

(event `Attack 3`
  ;[0.05098 0.05098 0.05098] Attack 3
  (`/Engine/EditorBlueprintResources/StandardMacros.DoOnce` false :!label _label_4
    (:`Completed`
      (`KismetSystemLibrary.Delay` 0.1)
      (`|PlayMontage` (`self.characterMesh`) "/Game/Animation/Sword_Attacks/Kick_Montage.Kick_Montage"
        (:`then`
          (set `self.attackIndex` 3)
          (goto _label_4 :!via `Reset`))))))

(event `Attack 4`
  ;[0.05098 0.05098 0.05098] Attack 4
  (`/Engine/EditorBlueprintResources/StandardMacros.DoOnce` false :!label _label_5
    (:`Completed`
      (`KismetSystemLibrary.Delay` 0.1)
      (`|PlayMontage` (`self.characterMesh`) "/Game/Animation/Sword_Attacks/Attack3_Montage.Attack3_Montage"
        (:`then`
          (set `self.attackIndex` 4)
          (goto _label_5 :!via `Reset`))))))